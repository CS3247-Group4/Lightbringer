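; BP_LightMirror is a mirror that reflects incoming light rays off its cube's forward vector and shows the reflected beams.
; Each emitter gets its own BPC_LightReceiver component, which receives the reflected ray and returns the end point for a paired Niagara beam.
; On Tick, any cube rotation change makes every receiver backtrack its ray.
; Removing a ray clears its map entries and beam, and the point light stays visible while receivers remain.
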(event EventRemoveLightRay
  (params (Receiver :type BPC%20Light%20Receiver%20Object%20Reference) (Emitter :type BPC%20Light%20Emitter%20Object%20Reference))
  (bind _receivermap (Variables|Default|GetReceiverMap))
  (bind _beammap (Variables|Default|GetBeamMap))
  (Default|RemoveLightRay Receiver)
  (Components|DestroyComponent (.Value (Utilities|Map|Find _beammap Receiver)))
  (Utilities|Map|Remove _beammap Receiver)
  (Utilities|Map|Remove _receivermap Emitter)
  (Utilities|ToggleLightComponent (> (Utilities|Map|Length _receivermap) 0)))

(event EventRemovePairedEmitters
  (params (Emitter :type BPC%20Light%20Emitter%20Object%20Reference))
  (Components|DestroyComponent Emitter))

(event EventTick
  (params (DeltaSeconds :type Float%20%28single-precision%29))
  (bind _cube (Variables|Default|GetCube))
  (bind _returnvalue (Transformation|GetWorldRotation _cube))
  ;[1 1 1] Check for Rotation
  (if (Utilities|Operators|NotEqual(!=) (Variables|Default|GetPrevRotation) _returnvalue 0.0)
    (Utilities|FlowControl|Sequence
      (:then_0
        (bind _values (Utilities|Map|Values (Variables|Default|GetReceiverMap)))
        (for _array_element _values
          (Default|BacktrackLightRay _array_element)))
      (:then_1
        (Variables|Default|SetPrevRotation _returnvalue)))))

(fn ConstructionScript)

(fn ReceiveLightRay
  (params (ImpactPoint :type Vector :default "0, 0, 0") (InDirection :type Vector :default "0, 0, 0") (Emitter :type BPC%20Light%20Emitter%20Object%20Reference))
  (LocalVariables|SetCurrentEmitter Emitter)
  (if (Utilities|Map|Contains (Variables|Default|GetReceiverMap) (LocalVariables|GetCurrentEmitter))
    _
    (else
      (bind _returnvalue (Game|AddComponentbyClass "/Game/Blueprints/LightComponents/BPC_LightReceiver.BPC_LightReceiver_C"))
      (Utilities|Map|Add (Variables|Default|GetReceiverMap) (LocalVariables|GetCurrentEmitter) _returnvalue)))
  (bind _pairedemitterend (Default|ReceiveLightRay (.Value (Utilities|Map|Find (Variables|Default|GetReceiverMap) (LocalVariables|GetCurrentEmitter))) (Utilities|Array|MakeArray ImpactPoint) (Utilities|Array|MakeArray (Math|Vector|GetReflectionVector InDirection (Math|Vector|GetForwardVector (Variables|Default|GetCube)))) (Variables|Default|GetReflectStrength) (LocalVariables|GetCurrentEmitter)))
  (Utilities|FlowControl|Sequence
    (:then_0
      (if (not (Utilities|Map|Contains (Variables|Default|GetBeamMap) (.Value (Utilities|Map|Find (Variables|Default|GetReceiverMap) (LocalVariables|GetCurrentEmitter)))))
        (bind _returnvalue_2 (AddComponent|AddNiagaraComponent false))
        (Utilities|Map|Add (Variables|Default|GetBeamMap) (.Value (Utilities|Map|Find (Variables|Default|GetReceiverMap) (LocalVariables|GetCurrentEmitter))) _returnvalue_2)
        (Class|NiagaraComponent|SetAsset _returnvalue_2 "/Game/VisualEffects/NS_LightBeam.NS_LightBeam" true)))
    (:then_1
      (Utilities|SetNiagaraBeam (Utilities|Array|Get(acopy) _pairedemitterend) ImpactPoint (.Value (Utilities|Map|Find (Variables|Default|GetBeamMap) (.Value (Utilities|Map|Find (Variables|Default|GetReceiverMap) (LocalVariables|GetCurrentEmitter)))))))
    (:then_2
      (Utilities|FlowControl|Sequence
        (:then_0
          (Utilities|ToggleLightComponent true))
        (:then_1
          (return (.Value (Utilities|Map|Find (Variables|Default|GetReceiverMap) (LocalVariables|GetCurrentEmitter)))))))))