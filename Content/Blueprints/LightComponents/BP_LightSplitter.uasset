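; BP_LightSplitter is a light-ray splitter that turns an incoming ray into paired emitters along two arrows.
; ReceiveLightRay adds a BPC_LightReceiver component as needed, passes it both arrows' positions and directions, fires the lit event and shows the point light.
; Tick tells the receiver to backtrack whenever the cube's rotation changes.
; Removing rays keeps the light visible while any tracked emitter remains.
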(event EventBeginPlay
  (Variables|Default|SetArrowList (Utilities|Array|MakeArray (Variables|Default|GetArrow1) (Variables|Default|GetArrow2))))

(event EventTick
  (params (DeltaSeconds :type Float%20%28single-precision%29))
  (bind _cube (Variables|Default|GetCube))
  (bind _returnvalue (Transformation|GetWorldRotation _cube))
  (if (Utilities|Operators|NotEqual(!=) (Variables|Default|GetPrevious%20Rotation) _returnvalue 0.0)
    (Utilities|FlowControl|Sequence
      (:then_0
        (if (Utilities|IsValid (Variables|Default|GetReceiver))
          (Default|BacktrackLightRay (Variables|Default|GetReceiver))))
      (:then_1
        (Variables|Default|SetPrevious%20Rotation _returnvalue)))))

(event EventRemovePairedEmitters
  (params (Emitter :type BPC%20Light%20Emitter%20Object%20Reference))
  (Components|DestroyComponent Emitter))

(event EventRemoveLightRay
  (params (Receiver :type BPC%20Light%20Receiver%20Object%20Reference) (Emitter :type BPC%20Light%20Emitter%20Object%20Reference))
  (bind _previousemitterlist (Variables|Default|GetPreviousEmitterList))
  (Default|RemoveLightRay Receiver)
  (Utilities|Array|RemoveItem _previousemitterlist Emitter)
  (Utilities|ToggleLightComponent (> (Utilities|Array|Length _previousemitterlist) 0)))

(fn ConstructionScript)

(fn ReceiveLightRay
  (params (ImpactPoint :type Vector :default "0, 0, 0") (InDirection :type Vector :default "0, 0, 0") (Emitter :type BPC%20Light%20Emitter%20Object%20Reference) (NumBounce :type Integer))
  (bind _previousemitterlist (Variables|Default|GetPreviousEmitterList))
  (bind _output_get (LocalVariables|SetCurrentEmitter Emitter))
  (Utilities|FlowControl|Sequence
    (:then_0
      (if (not (and (Utilities|IsValid (Variables|Default|GetReceiver)) (Utilities|Array|ContainsItem _previousemitterlist _output_get)))
        (bind _returnvalue (Game|AddComponentbyClass "/Game/Blueprints/LightComponents/BPC_LightReceiver.BPC_LightReceiver_C"))
        (Variables|Default|SetReceiver _returnvalue)))
    (:then_1
      (Utilities|Array|AddUnique _previousemitterlist _output_get))
    (:then_2
      (Default|ReceiveLightRay (Variables|Default|GetReceiver) NumBounce (Utilities|Array|MakeArray (Transformation|GetWorldLocation (Variables|Default|GetArrow1)) (Transformation|GetWorldLocation (Variables|Default|GetArrow2))) (Utilities|Array|MakeArray (Math|Vector|GetForwardVector (Variables|Default|GetArrow1)) (Math|Vector|GetForwardVector (Variables|Default|GetArrow2))) (Variables|Default|GetLight%20Range) (LocalVariables|GetCurrentEmitter))
      (Utilities|FlowControl|Sequence
        (:then_0
          (Default|CallOnSplitterLitEvent)
          (Utilities|ToggleLightComponent true))
        (:then_1
          (return (Variables|Default|GetReceiver)))))))