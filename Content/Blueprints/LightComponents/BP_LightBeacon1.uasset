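; BP_LightBeacon1 is a beacon that lights up when emitters send light rays to it.
; Receiving a ray records the emitter, forwards it to BPCLightReceiver, turns on the point light and the sphere's custom depth, and sets BeaconLit.
; Removing a ray notifies the receiver and drops the emitter, keeping the visuals on while any emitters remain.
; BeaconLit is never cleared here.
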(event EventRemoveLightRay
  (params (Receiver :type BPC%20Light%20Receiver%20Object%20Reference) (Emitter :type BPC%20Light%20Emitter%20Object%20Reference))
  (bind _emitterlist (Variables|Default|GetEmitterList))
  (Default|RemoveLightRay Receiver)
  (Utilities|Set|Remove _emitterlist Emitter)
  (Utilities|TogglePointLight (> (Utilities|Set|Length _emitterlist) 0)))

(fn ConstructionScript)

(fn ReceiveLightRay
  (params (ImpactPoint :type Vector :default "0, 0, 0") (InDirection :type Vector :default "0, 0, 0") (Emitter :type BPC%20Light%20Emitter%20Object%20Reference))
  (Utilities|FlowControl|Sequence
    (:then_0
      (Utilities|TogglePointLight true))
    (:then_1
      (Utilities|Set|Add (Variables|Default|GetEmitterList) Emitter)
      (Default|ReceiveLightRay (Variables|Default|GetBPC_LightReceiver) 0 0 0.0 Emitter)
      (Development|PrintString "Beacon Lit!")
      (Variables|Default|SetBeaconLit true))
    (:then_2
      (return 0))))