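; Light beacon that lights up when struck by light rays and fires an OnBeaconLit event.
; ReceiveLightRay records the emitter, creates a light receiver component if none is valid, forwards the emitter and returns that receiver.
; A point light and glowing sphere materials show the lit state.
; Any ray removal clears BeaconLit and the current receiver, but the glow persists while emitters remain.
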(event EventRemoveLightRay
  (params (Receiver :type BPC%20Light%20Receiver%20Object%20Reference) (Emitter :type BPC%20Light%20Emitter%20Object%20Reference))
  (bind _emitterlist (Variables|Default|GetEmitterList))
  (Utilities|FlowControl|Sequence
    (:then_0
      (Default|RemoveLightRay Receiver)
      (Variables|Default|SetBeaconLit false)
      (Utilities|Set|Remove _emitterlist Emitter)
      (Utilities|TogglePointLight (> (Utilities|Set|Length _emitterlist) 0)))
    (:then_1
      (Variables|Default|SetCurrentReceiver (Variables|Default|GetResetVal))
      (Development|PrintString "Hello" true true "(R=1.000000,G=0.378473,B=0.378473,A=1.000000)"))))

(fn ConstructionScript)

(fn ReceiveLightRay
  (params (ImpactPoint :type Vector :default "0, 0, 0") (InDirection :type Vector :default "0, 0, 0") (Emitter :type BPC%20Light%20Emitter%20Object%20Reference) (NumBounce :type Integer))
  (Utilities|FlowControl|Sequence
    (:then_0
      (Utilities|TogglePointLight true))
    (:then_1
      (Utilities|Set|Add (Variables|Default|GetEmitterList) Emitter)
      (if (and (> (Utilities|Set|Length (Variables|Default|GetEmitterList)) 0) (not (Utilities|IsValid (Variables|Default|GetCurrentReceiver))))
        (bind _returnvalue (Game|AddComponentbyClass "/Game/Blueprints/LightComponents/BPC_LightReceiver.BPC_LightReceiver_C"))
        (Variables|Default|SetCurrentReceiver _returnvalue)))
    (:then_2
      (Default|ReceiveLightRay (Variables|Default|GetCurrentReceiver) 0 0 0 0.0 Emitter)
      (Development|PrintString "Beacon Lit" true true "(R=1.000000,G=0.806797,B=0.000000,A=1.000000)")
      (Variables|Default|SetBeaconLit true)
      (Default|CallOnBeaconLitEvent))
    (:then_3
      (return (Variables|Default|GetCurrentReceiver)))))