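; BP_LightEmitter is an actor that emits a light ray in the game's light-beam system through its BPCLightEmitter component.
; On BeginPlay it initializes the component with a bounce limit, the Cube's world location and the LightRange variable, then sets the ray direction to the Cube's forward vector.
; Tick is empty, and a disconnected chain that would rotate the Cube and recompute the ray never runs.
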(event EventBeginPlay
  ;[1 1 1] Begin Play
  (Utilities|FlowControl|Sequence
    (:then_0
      (Default|EventInit (Variables|Default|GetBPC_LightEmitter) 25 (Transformation|GetWorldLocation (Variables|Default|GetCube)) (Variables|Default|GetLightRange)))
    (:then_1
      (Default|SetDirection (Variables|Default|GetBPC_LightEmitter) (Math|Vector|GetForwardVector (Variables|Default|GetCube))))))

(event EventTick
  (params (DeltaSeconds :type Float%20%28single-precision%29))
  ;[1 1 1] Raycast every frame until receiver is connected
)

(fn ConstructionScript)