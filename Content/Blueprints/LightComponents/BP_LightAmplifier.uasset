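; BP_LightAmplifier is a light-ray relay that re-emits incoming rays in the same direction using its own LightRange.
; Each incoming emitter gets a dynamically added BPC_LightReceiver, tracked in ReceiverMap, which receives the outgoing origin and direction.
; That origin is the impact point projected along the ray to the point nearest the Sphere's center.
; A PointLight shows on receiving a ray and hides once ReceiverMap empties.
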(event EventRemoveLightRay
  (params (Receiver :type BPC%20Light%20Receiver%20Object%20Reference) (Emitter :type BPC%20Light%20Emitter%20Object%20Reference))
  (bind _receivermap (Variables|Default|GetReceiverMap))
  (Default|RemoveLightRay Receiver)
  (Utilities|Map|Remove _receivermap Emitter)
  (Utilities|ToggleLightComponent (> (Utilities|Map|Length _receivermap) 0)))

(event EventRemovePairedEmitters
  (params (Emitter :type BPC%20Light%20Emitter%20Object%20Reference))
  (Components|DestroyComponent Emitter))

(fn ConstructionScript)

(fn ReceiveLightRay
  (params (ImpactPoint :type Vector :default "0, 0, 0") (InDirection :type Vector :default "0, 0, 0") (Emitter :type BPC%20Light%20Emitter%20Object%20Reference) (NumBounce :type Integer))
  (LocalVariables|SetCurrentEmitter Emitter)
  (if (Utilities|Map|Contains (Variables|Default|GetReceiverMap) (LocalVariables|GetCurrentEmitter))
    _
    (else
      (bind _returnvalue (Game|AddComponentbyClass "/Game/Blueprints/LightComponents/BPC_LightReceiver.BPC_LightReceiver_C"))
      (Utilities|Map|Add (Variables|Default|GetReceiverMap) (LocalVariables|GetCurrentEmitter) _returnvalue)))
  (Default|ReceiveLightRay (.Value (Utilities|Map|Find (Variables|Default|GetReceiverMap) (LocalVariables|GetCurrentEmitter))) NumBounce (Utilities|Array|MakeArray (+ ImpactPoint (* InDirection (Math|Float|Absolute(Float) (Math|Vector|DotProduct InDirection (- ImpactPoint (Transformation|GetWorldLocation (Variables|Default|GetSphere)))))))) (Utilities|Array|MakeArray InDirection) (Variables|Default|GetLight%20Range) (LocalVariables|GetCurrentEmitter))
  (Utilities|FlowControl|Sequence
    (:then_0
      (Utilities|ToggleLightComponent true))
    (:then_1
      (return (.Value (Utilities|Map|Find (Variables|Default|GetReceiverMap) (LocalVariables|GetCurrentEmitter)))))))