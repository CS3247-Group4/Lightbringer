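; Light emitter component that casts a directed light ray, shown as a Niagara beam, for a light-and-receiver mechanic.
; On tick it line-traces along its direction up to its range and moves the beam end to the hit or maximum range.
; Hit BPI_LightReceivers actors get the ray with its bounce count and return the connected receiver, which is notified when the ray leaves or is removed.
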(event Custom|Event%20Init
  (params (NumBounce :type Integer) (Location :type Vector) (Range :type Float%20%28double-precision%29))
  (Variables|Default|SetNumBounce NumBounce)
  (bind _output_get (Variables|Default|SetLocation Location))
  (Variables|Default|SetLightRange Range)
  (bind _returnvalue (Niagara|SpawnSystematLocation "/Game/VisualEffects/NS_LightBeam.NS_LightBeam" _output_get))
  (bind _output_get_2 (Variables|Default|SetLight%20Beam _returnvalue))
  (Niagara|SetNiagaraVariable(Float) _output_get_2 "Lifetime" 1.0))

(event Custom|Set%20Direction
  (params (Direction :type Vector))
  (Variables|Default|SetDirection Direction))

(event Custom|Set%20Location
  (params (Location :type Vector))
  (bind _output_get (Variables|Default|SetLocation Location))
  (Transformation|SetWorldLocation (Variables|Default|GetLight%20Beam) _output_get false true))

(event EventTick
  (params (DeltaSeconds :type Float%20%28single-precision%29))
  (CallFunction|ComputeLightRay))

(fn CheckRayHit
  (params (Direction :type Vector))
  (bind _lightrange (Variables|Default|GetLightRange))
  (bind _location (Variables|Default|GetLocation))
  (bind _returnvalue (* Direction _lightrange))
  (bind _returnvalue_2 (+ _location _returnvalue))
  (bind (_outhit _returnvalue_3) (Collision|LineTraceByChannel _location _returnvalue_2 "TraceTypeQuery1" false 0 "None"))
  (return _returnvalue_3 (select _returnvalue_3 (.ImpactPoint (Collision|BreakHitResult _outhit)) _returnvalue_2) (.HitActor (Collision|BreakHitResult _outhit))))

(fn ComputeLightRay
  (bind _direction (Variables|Default|GetDirection))
  (bind (_rayhit _endlocation _actorhit) (CallFunction|CheckRayHit _direction))
  (Utilities|FlowControl|Sequence
    (:then_0
      (if _rayhit
        (bind _asbpi_light_receivers (Utilities|Casting|CastToBPI_LightReceivers _actorhit)
          (:then
            (bind _receiver (Default|ReceiveLightRay _asbpi_light_receivers _endlocation _direction self (Variables|Default|GetNumBounce)))
            (Utilities|FlowControl|Sequence
              (:then_0
                (if (!= _receiver (Variables|Default|GetConnectedReceiver))
                  ;[1 1 1] Remove Light on receiver if not the same receiver or not a receiver
                  (if (Utilities|IsValid (Variables|Default|GetConnectedReceiver)) :!label _label
                    (Class|BPILightReceivers|RemoveLightRay(Message) (Components|GetOwner (Variables|Default|GetConnectedReceiver)) (Variables|Default|GetConnectedReceiver) self)
                    (Variables|Default|SetConnectedReceiver (LocalVariables|GetResetVal)))))
              (:then_1
                (Variables|Default|SetConnectedReceiver _receiver))))
          (:CastFailed
            (goto _label)))
        (else
          (goto _label))))
    (:then_1
      (Utilities|SetBeamEnd _endlocation))
    (:then_2
      (return _endlocation))))

(fn RemoveLightRay
  (bind _connectedreceiver (Variables|Default|GetConnectedReceiver))
  (Utilities|FlowControl|Sequence
    (:then_0
      (if (Utilities|IsValid _connectedreceiver)
        (Class|BPILightReceivers|RemoveLightRay(Message) (Components|GetOwner _connectedreceiver) _connectedreceiver self)))
    (:then_1
      (if (Utilities|IsValid (Variables|Default|GetLight%20Beam))
        (Development|SetHiddeninGame (Variables|Default|GetLight%20Beam) true true)
        (Niagara|SetNiagaraVariable(Float) (Variables|Default|GetLight%20Beam) "Lifetime" 0.0)
        (Variables|Default|SetLight%20Beam (Variables|Default|GetNSResetVal))))))

(fn BacktrackLightRay)