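; BP_HitBox is an invisible trigger box that signals when a Pawn overlaps it.
; Its Cube is hidden at BeginPlay, and a Pawn overlap calls the OnBoxHit dispatcher and prints a debug "Hello".
; A SetCollision event switches the Cube's collision between query-and-physics and none, so the box can be turned on or off.
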(event Custom|SetCollision
  (params (isCollisionEnabled :type Boolean))
  (if isCollisionEnabled
    (Collision|SetCollisionEnabled (Variables|Default|GetCube) "QueryAndPhysics")
    (else
      (Collision|SetCollisionEnabled (Variables|Default|GetCube) "NoCollision"))))

(event EventBeginPlay
  (Rendering|SetVisibility (Variables|Default|GetCube) false false))

(event Collision|EventActorBeginOverlap
  (params (OtherActor :type Actor%20Object%20Reference))
  (Utilities|Casting|CastToPawn OtherActor)
  (Default|CallOnBoxHit)
  (Development|PrintString "Hello"))

(event EventTick
  (params (DeltaSeconds :type Float%20%28single-precision%29)))

(fn ConstructionScript)