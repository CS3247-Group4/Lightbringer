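; Respawn checkpoint actor that registers itself as the player's last checkpoint when a VRSwimPawn_State enters its box.
; On overlap it writes itself to VRGameMode's LastRespawnCheckpoint and raises the indicator's emissive value through a dynamic material created in the construction script.
; At BeginPlay it caches the RespawnPoint component's world transform as RespawnedPosition.
; Nothing here resets the glow or performs the respawn.
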(event OnComponentBeginOverlap(Box)
  (params (OverlappedComponent :type Primitive%20Component%20Object%20Reference) (OtherActor :type Actor%20Object%20Reference) (OtherComp :type Primitive%20Component%20Object%20Reference) (OtherBodyIndex :type Integer) (bFromSweep :type Boolean) (SweepResult :type Hit%20Result%20Structure%20%28by%20ref%29))
  (Utilities|Casting|CastToVRSwimPawn_State OtherActor)
  (bind _asvrgame_mode (Utilities|Casting|CastToVRGameMode (Game|GetGameMode)))
  (Variables|/Game/VRTemplate/Blueprints/VRGameMode.VRGameMode_C|SetLastRespawnCheckpoint _asvrgame_mode self)
  (Rendering|Material|SetScalarParameterValue (Variables|Default|GetDMI) "EmissiveValue" 5.0 :!class /Script/Engine.MaterialInstanceDynamic))

(event EventBeginPlay
  (Variables|Default|SetRespawnedPosition (Transformation|GetWorldTransform (Variables|Default|GetRespawnPoint))))

(event Collision|EventActorBeginOverlap
  (params (OtherActor :type Actor%20Object%20Reference)))

(event EventTick
  (params (DeltaSeconds :type Float%20%28single-precision%29)))

(fn ConstructionScript
  (bind _returnvalue (Rendering|Material|CreateDynamicMaterialInstance (Variables|Default|GetCheckpointIndicator) 0 0 "None" :!class /Script/Engine.PrimitiveComponent))
  (Variables|Default|SetDMI _returnvalue))