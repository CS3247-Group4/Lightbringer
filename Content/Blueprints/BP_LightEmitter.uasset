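; BP_LightEmitter is a light emitter actor that projects a beam from its Cube along the cube's forward vector.
; On BeginPlay, CalculateLightRay sets the LightBeam effect's "Beam End" variable to a point LightRange ahead of the cube and prints a debug message.
; Tick compares the cube's world rotation to the stored previous rotation and recalculates only when it changes, with no trace or obstruction check.
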(event EventCalculateLightRay
  (bind _cube (Variables|Default|GetCube))
  (Class|NiagaraComponent|SetVariablePosition (Variables|Default|GetLightBeam) "Beam End" (+ (Transformation|GetWorldLocation _cube) (* (Variables|Default|GetLightRange) (Math|Vector|GetForwardVector _cube))))
  (Development|PrintString (Utilities|String|Append (Utilities|GetDisplayName (Variables|Default|GetDefaultSceneRoot)) ": Recalculate Light Ray")))

(event EventBeginPlay
  (CallFunction|CalculateLightRay))

(event EventTick
  (params (DeltaSeconds :type Float%20%28single-precision%29))
  (bind _cube (Variables|Default|GetCube))
  (bind _returnvalue (Transformation|GetWorldRotation _cube))
  (if (not (Utilities|Operators|EqualEqual _returnvalue (Variables|Default|GetPrevRotation) 0.0))
    (CallFunction|CalculateLightRay)
    (Variables|Default|SetPrevRotation _returnvalue)))

(fn ConstructionScript)