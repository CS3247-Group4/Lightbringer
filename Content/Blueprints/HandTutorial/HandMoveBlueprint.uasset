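; Tutorial Blueprint, apparently for a hand demonstration, that moves a referenced skeletal mesh's owning actor along a spline track.
; On BeginPlay, a Timeline plays at a rate set by Duration, starting from Offset.
; Each update maps the timeline alpha to distance along the spline and applies that world location and rotation to the actor.
; A second mesh's movement node and some vector math are left unconnected.
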(event EventBeginPlay
  (Variables|Default|Setlocation (Transformation|GetActorLocation (Components|GetOwner (Variables|Default|GetSkeletalMesh))))
  (Variables|Default|Setlocation1 (Transformation|GetActorLocation (Components|GetOwner (Variables|Default|GetSkeletalMesh1))))
  (Components|Timeline|SetPlayRate (Variables|Default|GetTimeline) (/ 1.0 (Variables|Default|Getduration)))
  (Components|Timeline|SetNewTime (Variables|Default|GetTimeline) (Variables|Default|Getoffset))
  (bind _newtrack_0 (Timeline|Timeline Play)
    (:Update
      (Variables|Default|Setalpha _newtrack_0)
      (Transformation|SetActorLocationAndRotation (Components|GetOwner (Variables|Default|GetSkeletalMesh)) (Spline|GetLocationatDistanceAlongSpline (Variables|/Game/Blueprints/HandTutorial/SplineBlueprint.SplineBlueprint_C|GetSpline (Variables|Default|Gettrack)) (Math|Float|Lerp 0.0 (Spline|GetSplineLength (Variables|/Game/Blueprints/HandTutorial/SplineBlueprint.SplineBlueprint_C|GetSpline (Variables|Default|Gettrack))) (Variables|Default|Getalpha)) "World") (Spline|GetRotationatDistanceAlongSpline (Variables|/Game/Blueprints/HandTutorial/SplineBlueprint.SplineBlueprint_C|GetSpline (Variables|Default|Gettrack)) (Math|Float|Lerp 0.0 (Spline|GetSplineLength (Variables|/Game/Blueprints/HandTutorial/SplineBlueprint.SplineBlueprint_C|GetSpline (Variables|Default|Gettrack))) (Variables|Default|Getalpha)) "World")))))

(event Collision|EventActorBeginOverlap
  (params (OtherActor :type Actor%20Object%20Reference)))

(event EventTick
  (params (DeltaSeconds :type Float%20%28single-precision%29)))

(fn ConstructionScript)