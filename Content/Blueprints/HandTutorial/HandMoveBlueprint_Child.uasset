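; HandMoveBlueprint_Child is a child Blueprint in the hand tutorial folder that keeps its actor positioned just below the player's camera.
; After running the parent Tick, it teleports itself every frame to the player camera manager's location with a fixed downward Z offset.
; It sets only location, and the construction script just calls the parent.
; BeginPlay and overlap events are disabled placeholders.
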(event EventBeginPlay
  (|CallParentFunction) ; This node is disabled and will not be called.\nDrag off pins to build functionality.
)

(event Collision|EventActorBeginOverlap
  (params (OtherActor :type Actor%20Object%20Reference))
  (|CallParentFunction OtherActor) ; This node is disabled and will not be called.\nDrag off pins to build functionality.
)

(event EventTick
  (params (DeltaSeconds :type Float%20%28single-precision%29))
  (bind _returnvalue (Game|GetPlayerCameraManager 0))
  (bind _returnvalue_2 (Transformation|GetActorLocation _returnvalue))
  (|CallParentFunction DeltaSeconds)
  (Transformation|SetActorLocation (Math|Vector|MakeVector (.x _returnvalue_2) (.y _returnvalue_2) (+ (.z _returnvalue_2) -4e+01)) false true))

(fn ConstructionScript
  (|CallParentFunction))