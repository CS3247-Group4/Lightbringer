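; BP_Checkpoint is a checkpoint marker actor that shows a widget pointing the player toward its static mesh.
; Each tick it moves the widget component to DistanceFromPlayer from the player camera along the direction to the mesh, then rotates it to face the camera.
; This keeps the world-space marker at a fixed distance from the view.
; On BeginPlay it passes the actor's location to the MarkerWidgetBlueprint as OriginalLocation.
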(event EventBeginPlay
  ;[1 1 1] Comment
  (bind _asmarker_widget_blueprint (Utilities|Casting|CastToMarkerWidgetBlueprint (UserInterface|GetWidget (Variables|Default|GetWidget))))
  (Variables|/Game/Blueprints/marker/MarkerWidgetBlueprint.MarkerWidgetBlueprint_C|SetOriginalLocation _asmarker_widget_blueprint (Transformation|GetActorLocation)))

(event Collision|EventActorBeginOverlap
  (params (OtherActor :type Actor%20Object%20Reference)))

(event EventTick
  (params (DeltaSeconds :type Float%20%28single-precision%29))
  (bind _returnvalue (Game|Player|GetPlayerPawn 0))
  (bind _widget (Variables|Default|GetWidget))
  (bind _returnvalue_2 (Actor|GetComponentbyClass _returnvalue "/Script/Engine.CameraComponent"))
  (bind _returnvalue_3 (Transformation|GetWorldLocation _returnvalue_2))
  ;[1 1 1] Comment
  (Transformation|SetWorldLocation _widget (+ (* (Math|Vector|GetUnitDirection(Vector) _returnvalue_3 (Transformation|GetWorldLocation (Variables|Default|GetStaticMesh))) (Variables|Default|GetdistanceFromPlayer)) _returnvalue_3) false false)
  (Transformation|SetWorldRotation _widget (Math|Rotator|FindLookatRotation (Transformation|GetWorldLocation _widget) _returnvalue_3) false false))

(fn ConstructionScript)