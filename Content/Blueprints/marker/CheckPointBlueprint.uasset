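; Checkpoint marker actor that displays a marker widget through its Widget component.
; On BeginPlay it passes the actor's location to the MarkerWidgetBlueprint as OriginalLocation.
; It then rotates the widget toward the player pawn's camera with a look-at rotation, set only once because Tick is unused.
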(event EventBeginPlay
  (bind _widget (Variables|Default|GetWidget))
  ;[1 1 1] Comment
  (bind _asmarker_widget_blueprint (Utilities|Casting|CastToMarkerWidgetBlueprint (UserInterface|GetWidget (Variables|Default|GetWidget))))
  (Variables|/Game/Blueprints/marker/MarkerWidgetBlueprint.MarkerWidgetBlueprint_C|SetOriginalLocation _asmarker_widget_blueprint (Transformation|GetActorLocation))
  ;[1 1 1] Comment
  (Transformation|SetWorldRotation _widget (Math|Rotator|FindLookatRotation (Transformation|GetWorldLocation _widget) (Transformation|GetWorldLocation (Actor|GetComponentbyClass (Game|Player|GetPlayerPawn 0) "/Script/Engine.CameraComponent"))) false false))

(event Collision|EventActorBeginOverlap
  (params (OtherActor :type Actor%20Object%20Reference)))

(event EventTick
  (params (DeltaSeconds :type Float%20%28single-precision%29)))

(fn ConstructionScript)