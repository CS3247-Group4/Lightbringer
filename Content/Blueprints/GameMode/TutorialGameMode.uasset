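; Game mode for the tutorial that respawns the VR thruster swim pawn.
; RespawnPlayer teleports the existing VRSwimPawn_Thruster to the respawn transform stored on LastRespawnCheckpoint, falling back to the PlayerStart when no valid checkpoint is set.
; Pawn and PlayerStart are found by class lookup, and debug strings are printed along the way.
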(event Custom|RespawnPlayer
  (Development|PrintString "Respawning player" true true "(R=0.000000,G=0.660000,B=1.000000,A=1.000000)" 5.0)
  (bind _lastrespawncheckpoint (Variables|Default|GetLastRespawnCheckpoint)
    (:then
      (Development|PrintString "valid checkpoint exists" true true "(R=0.000000,G=0.660000,B=1.000000,A=1.000000)" 5.0)
      (bind _returnvalue (Actor|GetActorOfClass "/Game/VRTemplate/Blueprints/VRSwimPawn_Thruster.VRSwimPawn_Thruster_C"))
      (Development|PrintString "game mode: pawn exists")
      (Transformation|Teleport _returnvalue (.Location (Math|Transform|BreakTransform (Variables|/Game/Blueprints/StateManagement/BP_RespawnCheckpoint.BP_RespawnCheckpoint_C|GetRespawnedPosition _lastrespawncheckpoint))) (.Rotation (Math|Transform|BreakTransform (Variables|/Game/Blueprints/StateManagement/BP_RespawnCheckpoint.BP_RespawnCheckpoint_C|GetRespawnedPosition _lastrespawncheckpoint))))
      (Development|PrintString (Utilities|String|Append "respawned at checkpoint " (Utilities|String|ToString(Transform) (Variables|/Game/Blueprints/StateManagement/BP_RespawnCheckpoint.BP_RespawnCheckpoint_C|GetRespawnedPosition _lastrespawncheckpoint))) true true "(R=0.000000,G=0.660000,B=1.000000,A=1.000000)" 5.0))
    (:else
      (Development|PrintString "no last checkpoint" true true "(R=0.000000,G=0.660000,B=1.000000,A=1.000000)" 5.0)
      (bind _returnvalue_2 (Actor|GetActorOfClass "/Script/Engine.PlayerStart"))
      (bind _returnvalue_3 (Actor|GetActorOfClass "/Game/VRTemplate/Blueprints/VRSwimPawn_Thruster.VRSwimPawn_Thruster_C"))
      (Transformation|Teleport _returnvalue_3 (.Location (Math|Transform|BreakTransform (Transformation|GetActorTransform _returnvalue_2))) (.Rotation (Math|Transform|BreakTransform (Transformation|GetActorTransform _returnvalue_2))))
      (Development|PrintString (Utilities|String|Append "respawned at player start " (Utilities|String|ToString(Transform) (Transformation|GetActorTransform _returnvalue_2))) true true "(R=0.000000,G=0.660000,B=1.000000,A=1.000000)" 5.0))))

(event EventBeginPlay)

(event EventTick
  (params (DeltaSeconds :type Float%20%28single-precision%29)))

(fn ConstructionScript)